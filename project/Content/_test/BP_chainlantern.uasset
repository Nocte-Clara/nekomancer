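; Test Blueprint for a chain lantern that procedurally builds a ten-link physics chain in its construction script; no lantern body is added in the graphs.
; Static mesh links are spaced along X, each rolled 90 degrees from the last, with damping and mass overrides to tune movement.
; Physics constraints between neighbouring links limit swing and twist and disable collision between each connected pair.
; The event graph holds no active logic.
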(fn `connectChainPhysics`
  (bind _chainlinks (`self.chainLinks`))
  (for _index (range (+ (- (`self.maxChainLinks`) 2) 1))
    (bind _output (`|GetArrayItem` (`self.physicsConstraints`) _index))
    (`PhysicsConstraintComponent.SetDisableCollision` _output true)
    (`PhysicsConstraintComponent.SetConstrainedComponents` _output (`|GetArrayItem` _chainlinks _index) "None" (`|GetArrayItem` _chainlinks (+ _index 1)) "None")))

(fn `createChainLinks`
  (for _index (range (`self.maxChainLinks`))
    (bind _returnvalue (`AddComponent|NODE_AddStaticMeshComponent-0` :`RelativeTransform` (`KismetMathLibrary.MakeTransform` (`KismetMathLibrary.MakeVector` (* _index 35.0)) (`KismetMathLibrary.MakeRotator` (* _index 90.0)) (`KismetMathLibrary.MakeVector` 15.0 15.0 15.0))))
    (`KismetArrayLibrary.Array_Set` (`self.chainLinks`) _index _returnvalue true)
    ;[0.04041 0.05405 0.15 0.5] chain movementspeed finetuning
    (`PrimitiveComponent.SetLinearDamping` _returnvalue 2.0)
    (`PrimitiveComponent.SetAngularDamping` _returnvalue 2.0)
    (`PrimitiveComponent.SetMassOverrideInKg` _returnvalue "None" 50.0 true)))

(fn `createPhysicsConstraints`
  (for _index (range (+ (- (`self.maxChainLinks`) 2) 1))
    (bind _returnvalue (`AddComponent|NODE_AddPhysicsConstraintComponent-1` :`RelativeTransform` (`KismetMathLibrary.MakeTransform` (`KismetMathLibrary.MakeVector` (+ (* _index 35.0) 18.0)) (`KismetMathLibrary.MakeRotator` (* _index 90.0)))))
    (`KismetArrayLibrary.Array_Set` (`self.physicsConstraints`) _index _returnvalue true)
    ;[0.04328 0.0427 0.15 0.5] chain to chain swinglimit finetuning
    (`PhysicsConstraintComponent.SetAngularSwing1Limit` _returnvalue "ACM_Limited" 30.0)
    (`PhysicsConstraintComponent.SetAngularSwing2Limit` _returnvalue "ACM_Limited" 30.0)
    (`PhysicsConstraintComponent.SetAngularTwistLimit` _returnvalue "ACM_Limited" 15.0)))

(fn `UserConstructionScript`
  (`|ExecutionSequence`
    (:`then_0`
      (set `self.maxChainLinks` 10))
    (:`then_1`
      (`self.createChainLinks`))
    (:`then_2`
      (`self.createPhysicsConstraints`))
    (:`then_3`
      (`self.connectChainPhysics`))))