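; Physics-driven lantern on a chain tethered to the player pawn's skeletal mesh, serving as a player light source.
; The construction script procedurally builds damped links, swing-limited constraints, the lantern and a PlayerLightSource component.
; It joins them link to link, ignoring Pawn collision on the first three links.
; Tick runs the light source's trace from the lantern, and MoveLantern pushes it upward and toward a goal.
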(event `self.ReceiveTick`
  (params (DeltaSeconds :type "Float (single-precision)"))
  (if true
    (`/Game/_test/playerLightSource.lightSourceObject` (`self.playerLightSource`) (`self.lantern`) 120.0 600.0 false)))

(fn `connectChainPhysics`
  (bind _playerphysicscontraint (`self.playerphysicsContraint`))
  (bind _chainlinks (`self.chainLinks`))
  (bind _returnvalue (- (`self.maxChainLinks`) 1))
  (for _index (range (+ _returnvalue 1))
    (bind _output (`|GetArrayItem` (`self.physicsConstraints`) _index))
    (`PhysicsConstraintComponent.SetDisableCollision` _output true)
    (if (!= _index _returnvalue)
      (bind _output_2 (`|GetArrayItem` _chainlinks _index))
      (`PhysicsConstraintComponent.SetConstrainedComponents` _output _output_2 "None" (`|GetArrayItem` _chainlinks (+ _index 1)) "None")
      (else
        (`PhysicsConstraintComponent.SetConstrainedComponents` _output _output_2 "None" (`self.lantern`) "None"))))
  (`PhysicsConstraintComponent.SetDisableCollision` _playerphysicscontraint true)
  (`PhysicsConstraintComponent.SetConstrainedComponents` _playerphysicscontraint (`|GetArrayItem` (`self.chainLinks`)) "None" (`|GetArrayItem` (`self.K2_GetComponentsByClass` (`GameplayStatics.GetPlayerPawn` 0) "/Script/Engine.SkeletalMeshComponent")) "None")
  (`PrimitiveComponent.SetCollisionResponseToChannel` (`|GetArrayItem` (`self.chainLinks`) 1) "ECC_Pawn" "ECR_Ignore")
  (`PrimitiveComponent.SetCollisionResponseToChannel` (`|GetArrayItem` (`self.chainLinks`)) "ECC_Pawn" "ECR_Ignore")
  (`PrimitiveComponent.SetCollisionResponseToChannel` (`|GetArrayItem` (`self.chainLinks`) 2) "ECC_Pawn" "ECR_Ignore"))

(fn `create Lantern`
  (bind _returnvalue (`AddComponent|NODE_AddStaticMeshComponent-1` :`RelativeTransform` (`KismetMathLibrary.MakeTransform` (`KismetMathLibrary.MakeVector` (* (`self.maxChainLinks`) 35.0) 0.0 -25.0) (struct) (`KismetMathLibrary.MakeVector` 0.5 0.5 0.5))))
  (set `self.lantern` _returnvalue))

(fn `createChainLinks`
  (for _index (range (`self.maxChainLinks`))
    (bind _returnvalue (`AddComponent|NODE_AddStaticMeshComponent-0` :`RelativeTransform` (`KismetMathLibrary.MakeTransform` (`KismetMathLibrary.MakeVector` (* _index 35.0)) (`KismetMathLibrary.MakeRotator` (* _index 90.0)) (`KismetMathLibrary.MakeVector` 15.0 15.0 15.0))))
    (`KismetArrayLibrary.Array_Set` (`self.chainLinks`) _index _returnvalue true)
    ;[0.04041 0.05405 0.15 0.5] chain movementspeed finetuning
    (`PrimitiveComponent.SetLinearDamping` _returnvalue 2.0)
    (`PrimitiveComponent.SetAngularDamping` _returnvalue 2.0)
    (`PrimitiveComponent.SetMassOverrideInKg` _returnvalue "None" 50.0 true)))

(fn `createPhysicsConstraints`
  (for _index (range (`self.maxChainLinks`))
    (bind _returnvalue (`AddComponent|NODE_AddPhysicsConstraintComponent-1` :`RelativeTransform` (`KismetMathLibrary.MakeTransform` (`KismetMathLibrary.MakeVector` (+ (* _index 35.0) 18.0)) (`KismetMathLibrary.MakeRotator` (* _index 90.0)))))
    (`KismetArrayLibrary.Array_Set` (`self.physicsConstraints`) _index _returnvalue true)
    ;[0.04328 0.0427 0.15 0.5] chain to chain swinglimit finetuning
    (`PhysicsConstraintComponent.SetAngularSwing1Limit` _returnvalue "ACM_Limited" 30.0)
    (`PhysicsConstraintComponent.SetAngularSwing2Limit` _returnvalue "ACM_Limited" 30.0)
    (`PhysicsConstraintComponent.SetAngularTwistLimit` _returnvalue "ACM_Limited" 15.0))
  (bind _returnvalue_2 (`AddComponent|NODE_AddPhysicsConstraintComponent-2` :`RelativeTransform` (`KismetMathLibrary.MakeTransform` (`KismetMathLibrary.MakeVector` (+ (* -1.0 35.0) 18.0)))))
  (bind _output_get (set `self.playerphysicsContraint` _returnvalue_2))
  ;[0.04328 0.0427 0.15 0.5] player physics constraints finetuning
  (`PhysicsConstraintComponent.SetAngularSwing1Limit` _output_get "ACM_Free" 0.0)
  (`PhysicsConstraintComponent.SetAngularSwing2Limit` _output_get "ACM_Limited" 30.0)
  (`PhysicsConstraintComponent.SetAngularTwistLimit` _output_get "ACM_Free" 15.0))

(fn `moveLantern`
  (params (goalLocation :type "Vector Structure"))
  (`PrimitiveComponent.AddForce` (`self.lantern`) (* (+ (`KismetMathLibrary.Normal` (`KismetMathLibrary.MakeVector` (.x (- goalLocation (`SceneComponent.GetSocketLocation` (`self.lantern`) "None"))) (.y (- goalLocation (`SceneComponent.GetSocketLocation` (`self.lantern`) "None"))))) (0.0 0.0 1.0)) 20000) "None" true))

(fn `UserConstructionScript`
  (`|ExecutionSequence`
    (:`then_0`
      (set `self.maxChainLinks` 12))
    (:`then_1`
      (`self.createChainLinks`))
    (:`then_2`
      (`self.createPhysicsConstraints`))
    (:`then_3`
      (`self.create Lantern`))
    (:`then_4`
      (`self.connectChainPhysics`))
    (:`then_5`
      (bind _returnvalue (`AddComponent|NODE_AddplayerLightSource-0`))
      (set `self.playerLightSource` _returnvalue))))