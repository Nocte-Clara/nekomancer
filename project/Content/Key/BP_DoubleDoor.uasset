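; BP_DoubleDoor is a two-panel door that opens only for a top-down character carrying a key.
; When a BP_TopDownCharacter overlaps its Box, it checks HasKey and either plays DoorTimeLine or prints a message that a key is needed.
; The timeline's DoorL and DoorR tracks drive the yaw of the Door1 and DoorR components as relative rotations.
; The file shows no closing logic.
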(event `self.Box.OnComponentBeginOverlap`
  (params (OverlappedComponent :type "PrimitiveComponent Object Reference") (OtherActor :type "Actor Object Reference") (OtherComp :type "PrimitiveComponent Object Reference") (OtherBodyIndex :type Integer) (bFromSweep :type Boolean) (SweepResult :type "HitResult Structure (by ref)"))
  (bind _asbp_top_down_character (cast `/Game/TopDown/Blueprints/BP_TopDownCharacter` OtherActor))
  (if (`/Game/TopDown/Blueprints/BP_TopDownCharacter.hasKey` _asbp_top_down_character)
    (bind (_direction _doorl _doorr_) (`Timeline|DoorTimeLine`)
      (:`Update`
        (bind _output_get (set `self.DoorL_RelativeRotation_0` _doorl))
        (bind _output_get_2 (set `self.DoorR_RelativeRotation` _doorr_))
        (`SceneComponent.K2_SetRelativeRotation` (`self.doorR`) (`KismetMathLibrary.MakeRotator` 0.0 0.0 (.z _output_get_2)) false false)
        (`SceneComponent.K2_SetRelativeRotation` (`self.door1`) (`KismetMathLibrary.MakeRotator` 0.0 0.0 (.z _output_get)) false false)))
    (else
      (`KismetSystemLibrary.PrintString` "You need a key to open the door"))))

(fn `UserConstructionScript`)